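; Main menu camera that flies to one of four in-world screens when clicked and zooms back out on request.
; A mouse-position trace finds actors tagged "Camera Target", and their class selects the screen number and stored destination transform.
; A timeline lerps the camera there, then the screen's text hides and its menu widget appears.
; ZoomOutCamera removes widgets, restores all screen texts, lerps back to the saved start and unlocks clicking.
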(event `self.ReceiveBeginPlay`
  (bind _camera (`self.Camera`))
  ;[1 1 1] Saving Starting Camera
  (set `self.Camera Start` (`KismetMathLibrary.MakeTransform` (`SceneComponent.RelativeLocation` _camera) (`SceneComponent.RelativeRotation` _camera))))

(event `Key|LeftMouseButton`
  (params (Key :type "Key Structure"))
  (bind (_camera_destination_location _camera_destination_rotation) (`KismetMathLibrary.BreakTransform` (`self.Camera Destination`)))
  (bind (_camera_start_location _camera_start_rotation) (`KismetMathLibrary.BreakTransform` (`self.Camera Start`)))
  (bind (_worldlocation _worlddirection) (`PlayerController.DeprojectMousePositionToWorld` (`GameplayStatics.GetPlayerController` 0)))
  (:`Pressed`
    (bind _outhit (`KismetSystemLibrary.LineTraceSingle` _worldlocation (+ _worldlocation (* _worlddirection 10000.0)) "TraceTypeQuery1"))
    (if (`KismetArrayLibrary.Array_Contains` (`Actor.Tags` (`.HitActor` (`GameplayStatics.BreakHitResult` _outhit))) "Camera Target")
      (`self.CheckWhichScreenClicked` (`.HitActor` (`GameplayStatics.BreakHitResult` _outhit)))
      (if (not (`self.Locked To Screen`))
        (set `self.Locked To Screen` true)
        (bind (_direction _default) (`Timeline|Camera Move` :!via `PlayFromStart`)
          (:`Update`
            (`SceneComponent.K2_SetRelativeLocationAndRotation` (`self.Camera`) (`KismetMathLibrary.VLerp` _camera_start_location _camera_destination_location _default) (`KismetMathLibrary.RLerp` _camera_start_rotation _camera_destination_rotation _default) false false)
            (`KismetSystemLibrary.Delay` 1.0)
            (if (== (`self.Screen Number`) 1)
              (bind _returnvalue (`GameplayStatics.GetActorOfClass` "/Game/FirstPerson/MainMenu/BP_Screen01.BP_Screen01_C"))
              (`SceneComponent.SetVisibility` (`/Game/FirstPerson/MainMenu/BP_Screen01.TextRender` _returnvalue) false false)
              (bind _returnvalue_2 (`|CreateWidget` "/Game/FirstPerson/MainMenu/BW_MM_Start.BW_MM_Start_C"))
              (`UserWidget.AddToViewport` _returnvalue_2 0)
              (elif (== (`self.Screen Number`) 2)
                (bind _returnvalue_3 (`GameplayStatics.GetActorOfClass` "/Game/FirstPerson/MainMenu/BP_Screen02.BP_Screen02_C"))
                (`SceneComponent.SetVisibility` (`/Game/FirstPerson/MainMenu/BP_Screen02.Options Text` _returnvalue_3) false false)
                (bind _returnvalue_4 (`|CreateWidget` "/Game/FirstPerson/MainMenu/BW_MM_Options.BW_MM_Options_C"))
                (`UserWidget.AddToViewport` _returnvalue_4 0)
                (elif (== (`self.Screen Number`) 3)
                  (bind _returnvalue_5 (`GameplayStatics.GetActorOfClass` "/Game/FirstPerson/MainMenu/BP_Screen03.BP_Screen03_C"))
                  (`SceneComponent.SetVisibility` (`/Game/FirstPerson/MainMenu/BP_Screen03.Stats text` _returnvalue_5) false false)
                  (bind _returnvalue_6 (`|CreateWidget` "/Game/FirstPerson/MainMenu/BW_MM_Stats.BW_MM_Stats_C"))
                  (`UserWidget.AddToViewport` _returnvalue_6 0)
                  (elif (== (`self.Screen Number`) 4)
                    (bind _returnvalue_7 (`GameplayStatics.GetActorOfClass` "/Game/FirstPerson/MainMenu/BP_Screen04.BP_Screen04_C"))
                    (`SceneComponent.SetVisibility` (`/Game/FirstPerson/MainMenu/BP_Screen04.Credits Text` _returnvalue_7) false false)
                    (bind _returnvalue_8 (`|CreateWidget` "/Game/FirstPerson/MainMenu/BW_MM_Credits.BW_MM_Credits_C"))
                    (`UserWidget.AddToViewport` _returnvalue_8 0)))))))))))

(event `Zoom Out Camera`
  (bind (_camera_start_location _camera_start_rotation) (`KismetMathLibrary.BreakTransform` (`self.Camera Start`)))
  (bind (_camera_destination_location _camera_destination_rotation) (`KismetMathLibrary.BreakTransform` (`self.Camera Destination`)))
  ;[1 1 1] Zoom Out of Screens
  (`WidgetLayoutLibrary.RemoveAllWidgets`)
  (`|ExecutionSequence`
    (:`then_0`
      (bind _returnvalue (`GameplayStatics.GetActorOfClass` "/Game/FirstPerson/MainMenu/BP_Screen01.BP_Screen01_C"))
      (`SceneComponent.SetVisibility` (`/Game/FirstPerson/MainMenu/BP_Screen01.TextRender` _returnvalue) true false))
    (:`then_1`
      (bind _returnvalue_2 (`GameplayStatics.GetActorOfClass` "/Game/FirstPerson/MainMenu/BP_Screen02.BP_Screen02_C"))
      (`SceneComponent.SetVisibility` (`/Game/FirstPerson/MainMenu/BP_Screen02.Options Text` _returnvalue_2) true false))
    (:`then_2`
      (bind _returnvalue_3 (`GameplayStatics.GetActorOfClass` "/Game/FirstPerson/MainMenu/BP_Screen03.BP_Screen03_C"))
      (`SceneComponent.SetVisibility` (`/Game/FirstPerson/MainMenu/BP_Screen03.Stats text` _returnvalue_3) true false))
    (:`then_3`
      (bind _returnvalue_4 (`GameplayStatics.GetActorOfClass` "/Game/FirstPerson/MainMenu/BP_Screen04.BP_Screen04_C"))
      (`SceneComponent.SetVisibility` (`/Game/FirstPerson/MainMenu/BP_Screen04.Credits Text` _returnvalue_4) true false)))
  (if (`self.Locked To Screen`)
    (bind (_direction _default) (`Timeline|Timeline` :!via `PlayFromStart`)
      (:`Update`
        (`SceneComponent.K2_SetRelativeLocationAndRotation` (`self.Camera`) (`KismetMathLibrary.VLerp` _camera_destination_location _camera_start_location _default) (`KismetMathLibrary.RLerp` _camera_destination_rotation _camera_start_rotation _default) false false)
        (`KismetSystemLibrary.Delay` 1.0)
        (set `self.Locked To Screen` false)))))

(fn `CheckIfClickedOnScreen`
  (params (self2 :type "Actor Object Reference") (Condition :type Boolean))
  (if Condition
    (if (`KismetArrayLibrary.Array_Contains` (`Actor.Tags` self2) "ClickableScreen")
      _)))

(fn `CheckWhichScreenClicked`
  (params (Object :type "Object Object Reference"))
  (bind _returnvalue (`GameplayStatics.GetObjectClass` Object))
  (bind (_screen03_transform_location _screen03_transform_rotation) (`KismetMathLibrary.BreakTransform` (`self.Screen03 Transform`)))
  (bind (_screen04_transform_location _screen04_transform_rotation) (`KismetMathLibrary.BreakTransform` (`self.Screen04 Transform`)))
  (bind (_screen01_transform_location _screen01_transform_rotation) (`KismetMathLibrary.BreakTransform` (`self.Screen01 Transform`)))
  (bind (_screen02_transform_location _screen02_transform_rotation) (`KismetMathLibrary.BreakTransform` (`self.Screen02 Transform`)))
  (if (== _returnvalue "/Game/FirstPerson/MainMenu/BP_Screen01.BP_Screen01_C")
    (set `self.Screen Number` 1)
    (set `self.Camera Destination` (`KismetMathLibrary.MakeTransform` _screen01_transform_location _screen01_transform_rotation))
    (elif (== _returnvalue "/Game/FirstPerson/MainMenu/BP_Screen02.BP_Screen02_C")
      (set `self.Screen Number` 2)
      (set `self.Camera Destination` (`KismetMathLibrary.MakeTransform` _screen02_transform_location _screen02_transform_rotation))
      (elif (== _returnvalue "/Game/FirstPerson/MainMenu/BP_Screen03.BP_Screen03_C")
        (set `self.Screen Number` 3)
        (set `self.Camera Destination` (`KismetMathLibrary.MakeTransform` _screen03_transform_location _screen03_transform_rotation))
        (elif (== _returnvalue "/Game/FirstPerson/MainMenu/BP_Screen04.BP_Screen04_C")
          (set `self.Screen Number` 4)
          (set `self.Camera Destination` (`KismetMathLibrary.MakeTransform` _screen04_transform_location _screen04_transform_rotation)))))))

(fn `UserConstructionScript`)