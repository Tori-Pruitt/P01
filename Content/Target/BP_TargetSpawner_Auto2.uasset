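; Automatic target spawner that keeps the level populated with BP_Target actors inside a box volume.
; BeginPlay spawns an initial batch and starts a looping timer that adds one target per tick while the world-wide target count is within a small cap.
; Each target appears at a random point in SpawnArea, rotated toward SpawnAim with a yaw offset.
; The construction script sizes SpawnArea from the BoxExtent variable.
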(event `self.ReceiveBeginPlay`
  (`KismetSystemLibrary.K2_SetTimerDelegate` (delegate `SpawnTarget`) 1.0 true)
  (for _ (range 9)
    (`self.SpawnTarget`)))

(event `SpawnTarget`
  (bind _spawn_area (`self.Spawn Area`))
  (bind _outactors (`GameplayStatics.GetAllActorsOfClass` "/Game/FirstPerson/Blueprints/Target/BP_Target.BP_Target_C"))
  (if (<= (`KismetArrayLibrary.Array_Length` _outactors) 10)
    (bind _output_get (set `self.SpawnLocation` (`KismetMathLibrary.RandomPointInBoundingBox` (`SceneComponent.K2_GetComponentLocation` _spawn_area) (`BoxComponent.GetScaledBoxExtent` _spawn_area))))
    (bind (_returnvalue_roll _returnvalue_pitch _returnvalue_yaw) (`KismetMathLibrary.BreakRotator` (`KismetMathLibrary.FindLookAtRotation` _output_get (`SceneComponent.K2_GetComponentLocation` (`self.Spawn Aim`)))))
    (`|SpawnActorFromClass` "/Game/FirstPerson/Blueprints/Target/BP_Target.BP_Target_C" (`KismetMathLibrary.MakeTransform` _output_get (`KismetMathLibrary.MakeRotator` _returnvalue_roll _returnvalue_pitch (- _returnvalue_yaw 90.0))) "AdjustIfPossibleButAlwaysSpawn" "MultiplyWithRoot" null null)))

(fn `UserConstructionScript`
  (`BoxComponent.SetBoxExtent` (`self.Spawn Area`) (`self.BoxExtent`) true))