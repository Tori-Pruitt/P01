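; Main menu camera Blueprint that detects left clicks on in-world screens, such as a computer.
; Each click deprojects the mouse position and runs a long line trace on the Visibility channel.
; A hit actor tagged ClickableScreen only prints a debug message; the branch after it is empty, so no menu action or camera movement happens yet.
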(event `Key|LeftMouseButton`
  (params (Key :type "Key Structure"))
  (bind (_worldlocation _worlddirection) (`PlayerController.DeprojectMousePositionToWorld` (`GameplayStatics.GetPlayerController` 0)))
  (:`Pressed`
    (bind (_outhit _returnvalue) (`KismetSystemLibrary.LineTraceSingle` _worldlocation (+ _worldlocation (* _worlddirection 10000.0)) "TraceTypeQuery1"))
    (if _returnvalue
      (`|ExecutionSequence`
        (:`then_0`
          (if (`KismetArrayLibrary.Array_Contains` (`Actor.Tags` (`.HitActor` (`GameplayStatics.BreakHitResult` _outhit))) "ClickableScreen")
            (`KismetSystemLibrary.PrintString` "Mouse On Computer")
            (if true
              _)))))))

(fn `UserConstructionScript`)