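; Base weapon Blueprint that tracks ammo, plays muzzle particle and sound effects on firing, and exposes an FOV multiplier.
; Fire triggers a reload when ammo is empty, otherwise decrements it, runs effects and calls WeaponTrace, an empty event here.
; Reloading shows a progress-bar widget and waits ReloadTime, but then assigns MaxAmmo to itself, leaving Ammo unrefilled.
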(event `self.ReceiveBeginPlay`
  (set `self.Ammo` (`self.MaxAmmo`)))

(event `ReloadWeapon`
  (bind _reloadtime (`self.ReloadTime`))
  (bind _returnvalue (`|CreateWidget` "/Game/FirstPerson/Blueprints/Weapons/WB_ReloadBar.WB_ReloadBar_C" :!label _label))
  (`/Game/FirstPerson/Blueprints/Weapons/WB_ReloadBar.Reload Animation` _returnvalue _reloadtime)
  (`UserWidget.AddToViewport` _returnvalue 0)
  (`KismetSystemLibrary.Delay` _reloadtime)
  (set `self.MaxAmmo` (`self.MaxAmmo`)))

(event `/Game/FirstPerson/Blueprints/Weapons/BPI_Weapon.Reload`
  (goto _label))

(event `/Game/FirstPerson/Blueprints/Weapons/BPI_Weapon.Fire`
  (bind _ammo (`self.Ammo`))
  (`KismetSystemLibrary.PrintString` "Fired")
  (`/Game/FirstPerson/Blueprints/Libraries/BPML_Comparisons.INT<=INT` _ammo
    (:`True`
      (`self.ReloadWeapon`))
    (:`False`
      (set `self.Ammo` (- _ammo 1))
      (`self.WeaponFireEffects`)
      (`self.Weapon Trace`)
      (`/Game/FirstPerson/Blueprints/Libraries/BPML_Comparisons.INT<=INT` (`self.Ammo`)
        (:`True`
          (`self.ReloadWeapon`))))))

(event `Weapon Trace`)

(fn `GetFOVMultiplier`
  (returns (FOVMultiplier :type "Float (double-precision)"))
  (return (`self.FOVMultiplier`)))

(fn `UserConstructionScript`)

(fn `WeaponFireEffects`
  (bind (_returnvalue_location _returnvalue_rotation) (`KismetMathLibrary.BreakTransform` (`SceneComponent.K2_GetComponentToWorld` (`self.Muzzle`))))
  (`GameplayStatics.SpawnEmitterAtLocation` (`self.WeaponFireEmitter`) _returnvalue_location _returnvalue_rotation (`self.WeaponFireScale`))
  (`GameplayStatics.SpawnSoundAtLocation` (`self.WeaponFireSound`) _returnvalue_location (struct) 1.0 1.0 0.0 null null)
  (return))